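; Trigger box that rolls for random monster encounters while the third-person character is inside it.
; Overlap starts a looping roll timer after a short delay, and leaving pauses it.
; Each failed roll raises the next chance; success resets the count, pauses the timer and picks a weighted encounter from PossibleEncounters' Area1 map.
; The MonsterManager lookup that follows is unfinished: its loop is empty, so nothing spawns here.
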(event Custom|RollForEncounter
  (if (Math|Random|RandomBoolwithWeight (+ (Math|Float|MakeLiteralFloat 0.1) (* (Variables|Default|GetTimesRollFailed) 0.05)))
    (Variables|Default|SetTimesRollFailed 0)
    (Utilities|Time|PauseTimerbyHandle (Variables|Default|GetSpawnTimer))
    (CallFunction|SetEncounterArray)
    (else
      (Math|Integer|IncrementInt (Variables|Default|GetTimesRollFailed)))))

(event Custom|SetEncounterArray
  (bind _selectedencounter (CallFunction|RollEncounter))
  (bind _outactors (Actor|GetAllActorsOfClass "/Game/EnemyPrefabs/MonsterManager.MonsterManager_C"))
  (for _array_element _outactors
    _))

(event EventBeginPlay)

(event Collision|EventActorBeginOverlap
  (params (OtherActor :type Actor%20Object%20Reference))
  (Utilities|Casting|CastToThirdPersonCharacter OtherActor)
  (Utilities|FlowControl|Delay 1.0)
  (Variables|Default|SetInRange true)
  (bind _returnvalue (Utilities|Time|SetTimerbyEvent (delegate Custom|RollForEncounter) 0.5 true))
  (Variables|Default|SetSpawnTimer _returnvalue))

(event EventTick
  (params (DeltaSeconds :type Float%20%28single-precision%29)))

(event Collision|EventActorEndOverlap
  (params (OtherActor :type Actor%20Object%20Reference))
  (Utilities|Casting|CastToThirdPersonCharacter OtherActor)
  (Utilities|FlowControl|Delay 1.0)
  (Variables|Default|SetInRange false)
  (Utilities|Time|PauseTimerbyHandle (Variables|Default|GetSpawnTimer)))

(fn ConstructionScript)

(fn RollEncounter
  (bind _possibleencounters (Variables|Default|GetPossibleEncounters))
  (bind _area1 (Utilities|Struct|BreakBP_PossibleEncounters _possibleencounters))
  (Variables|Default|SetSumofArrays 0.0)
  (bind _values (Utilities|Map|Values (Utilities|Struct|BreakBP_PossibleEncounters (Variables|Default|GetPossibleEncounters))))
  (for _array_element _values
    (Variables|Default|SetSumofArrays (+ _array_element (Variables|Default|GetSumofArrays))))
  (Variables|Default|SetRoll (Math|Random|RandomFloatinRange 0.0 (Variables|Default|GetSumofArrays)))
  (bind _keys (Utilities|Map|Keys _area1))
  (bind _array_element_2 (Utilities|Array|ForEachLoopwithBreak _keys :!label _label)
    (:LoopBody
      (if (>= (.Value (Utilities|Map|Find _area1 _array_element_2)) (Variables|Default|GetRoll))
        (Variables|Default|SetSelectedEncounter _array_element_2)
        (goto _label Break)
        (else
          (Variables|Default|SetRoll (- (Variables|Default|GetRoll) (.Value (Utilities|Map|Find _area1 _array_element_2)))))))
    (:Completed
      (return (Variables|Default|GetSelectedEncounter)))))