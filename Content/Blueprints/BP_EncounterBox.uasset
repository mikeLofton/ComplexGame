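; BP_EncounterBox is a trigger volume that tracks when the ThirdPersonCharacter is inside an encounter area.
; Its Box overlap events set or clear an Inrange flag, each after a short delay.
; On entry, it also loops over all MonsterManager actors and prints whether each MonsterInfo name matches the first EncounterList entry.
; That comparison only produces debug text, and nothing is spawned or started here.
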(event OnComponentBeginOverlap(Box)
  (params (OverlappedComponent :type Primitive%20Component%20Object%20Reference) (OtherActor :type Actor%20Object%20Reference) (OtherComp :type Primitive%20Component%20Object%20Reference) (OtherBodyIndex :type Integer) (bFromSweep :type Boolean) (SweepResult :type Hit%20Result%20Structure%20%28by%20ref%29))
  (Utilities|Casting|CastToThirdPersonCharacter OtherActor)
  (Utilities|FlowControl|Delay 1.0)
  (Variables|Default|SetInrange true)
  (bind _outactors (Actor|GetAllActorsOfClass "/Game/EnemyPrefabs/MonsterManager.MonsterManager_C"))
  (for _array_element _outactors
    (Development|PrintString (Utilities|String|ToString(Boolean) (== (.Name (Utilities|Struct|BreakMonsterStruct (Variables|/Game/EnemyPrefabs/MonsterManager.MonsterManager_C|GetMonsterInfo _array_element))) (Math|Conversions|ToByte(Integer) (Math|Conversions|ToInteger(Byte) (.Encounter1 (Utilities|Struct|BreakArea1 (Variables|Default|GetEncounterList))))))))))

(event OnComponentEndOverlap(Box)
  (params (OverlappedComponent :type Primitive%20Component%20Object%20Reference) (OtherActor :type Actor%20Object%20Reference) (OtherComp :type Primitive%20Component%20Object%20Reference) (OtherBodyIndex :type Integer))
  (Utilities|Casting|CastToThirdPersonCharacter OtherActor)
  (Utilities|FlowControl|Delay 0.2)
  (Variables|Default|SetInrange false))

(fn ConstructionScript)